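; BP_GlassFloor is a pair of left and right glass panels where one is solid and the other has no collision.
; BeginPlay calls a server event that rolls a random number into the RepNotify variable RandomChance.
; Its OnRep picks the solid side with even odds and assigns collision or no-collision static meshes to the matching components.
; The right panel always takes the opposite of the left, with broken flags tracking the fake side.
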(event Custom|SERVER_RandomChance
  (Variables|Default|SetRandomChance (Math|Random|RandomInteger 10)))

(event Custom|SpawnStaticMesh
  (Components|StaticMesh|SetStaticMesh (Variables|Default|GetLeftCollisionGlass) "/Game/Assets/Meshes/GlassFloor/SM_GlassFloor.SM_GlassFloor")
  (if (Variables|Default|GetisLeftFloorBroken)
    (Components|StaticMesh|SetStaticMesh (Variables|Default|GetRightCollisionGlass) "/Game/Assets/Meshes/GlassFloor/SM_GlassFloor.SM_GlassFloor")
    (else
      (Components|StaticMesh|SetStaticMesh (Variables|Default|GetRightNoCollisionGlass) "/Game/Assets/Meshes/GlassFloor/SM_GlassFloorNoCollision.SM_GlassFloorNoCollision")
      (Variables|Default|SetisRightFloorBroken true))))

(event Custom|SpawnDestructibleMesh
  (Components|StaticMesh|SetStaticMesh (Variables|Default|GetLeftNoCollisionGlass) "/Game/Assets/Meshes/GlassFloor/SM_GlassFloorNoCollision.SM_GlassFloorNoCollision")
  (Variables|Default|SetisLeftFloorBroken true)
  (if (Variables|Default|GetisLeftFloorBroken)
    (Components|StaticMesh|SetStaticMesh (Variables|Default|GetRightCollisionGlass) "/Game/Assets/Meshes/GlassFloor/SM_GlassFloor.SM_GlassFloor")
    (else
      (Components|StaticMesh|SetStaticMesh (Variables|Default|GetRightNoCollisionGlass) "/Game/Assets/Meshes/GlassFloor/SM_GlassFloorNoCollision.SM_GlassFloorNoCollision")
      (Variables|Default|SetisRightFloorBroken true))))

(event EventBeginPlay
  (CallFunction|SERVERRandomChance))

(fn ConstructionScript)

(fn OnRepRandomChance
  (if (>= (Variables|Default|GetRandomChance) 5)
    (CallFunction|SpawnStaticMesh)
    (else
      (CallFunction|SpawnDestructibleMesh))))