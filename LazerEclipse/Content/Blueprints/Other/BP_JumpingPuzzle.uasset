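; Glass-floor jumping puzzle actor that sets up colored answer markers showing which side of each of six glass pairs is safe.
; On BeginPlay it loops over six BP_GlassFloor child actors, matching each to its left and right answer components by index.
; SetAnswerColors reads each floor's left and right broken flags, giving the broken side's marker the wrong material and the other the correct one.
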(event EventBeginPlay
  (for (_array_element _array_index) (Utilities|Array|MakeArray (Variables|Default|GetGlasses1) (Variables|Default|GetGlasses2) (Variables|Default|GetGlasses3) (Variables|Default|GetGlasses4) (Variables|Default|GetGlasses5) (Variables|Default|GetGlasses6))
    (CallFunction|SetAnswerColors _array_element (Utilities|Select :Index _array_index :Option%200 (Variables|Default|GetGlasses1LeftAnswer) :Option%201 (Variables|Default|GetGlasses2LeftAnswer) :Option%202 (Variables|Default|GetGlasses3LeftAnswer) :Option%203 (Variables|Default|GetGlasses4LeftAnswer) :Option%204 (Variables|Default|GetGlasses5LeftAnswer) :Option%205 (Variables|Default|GetGlasses6LeftAnswer)) (Utilities|Select :Index _array_index :Option%200 (Variables|Default|GetGlasses1RightAnswer) :Option%201 (Variables|Default|GetGlasses2RightAnswer) :Option%202 (Variables|Default|GetGlasses3RightAnswer) :Option%203 (Variables|Default|GetGlasses4RightAnswer) :Option%204 (Variables|Default|GetGlasses5RightAnswer) :Option%205 (Variables|Default|GetGlasses6RightAnswer)) "/Engine/MapTemplates/Materials/BasicAsset03.BasicAsset03" "/Engine/MapTemplates/Materials/BasicAsset01.BasicAsset01")))

(fn ConstructionScript)

(fn SetAnswerColors
  (params (GlassReference :type Child%20Actor%20Component%20Object%20Reference) (LeftAnswerReference :type Static%20Mesh%20Component%20Object%20Reference) (RightAnswerReference :type Static%20Mesh%20Component%20Object%20Reference) (CorrectFloorMaterial :type Material%20Interface%20Object%20Reference) (WrongFloorMateiral :type Material%20Interface%20Object%20Reference))
  (bind _asbp_glass_floor (Utilities|Casting|CastToBP_GlassFloor (Variables|/Script/Engine.ChildActorComponent|GetChildActor GlassReference)))
  (Utilities|FlowControl|Sequence
    (:then_0
      (if (Variables|/Game/Blueprints/Other/BP_GlassFloor.BP_GlassFloor_C|GetisLeftFloorBroken _asbp_glass_floor)
        (Rendering|Material|SetMaterial LeftAnswerReference 0 WrongFloorMateiral)
        (Rendering|Material|SetMaterial RightAnswerReference 0 CorrectFloorMaterial)))
    (:then_1
      (if (Variables|/Game/Blueprints/Other/BP_GlassFloor.BP_GlassFloor_C|GetisRightFloorBroken _asbp_glass_floor)
        (Rendering|Material|SetMaterial RightAnswerReference 0 WrongFloorMateiral)
        (Rendering|Material|SetMaterial LeftAnswerReference 0 CorrectFloorMaterial)))
    (:then_2
      (return))))